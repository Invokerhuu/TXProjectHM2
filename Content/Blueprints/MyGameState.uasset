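; Game state Blueprint that runs a timed round and shows the game over menu when time runs out.
; GameStart sets a 15-second Timer and starts a looping one-second CountDown that decrements it down to zero.
; Tick polls for expiry while GameIsStart is true, then adds the GameOverMenu widget, shows the mouse cursor and clears the flag so it fires once.
; Both OnRep functions are empty.
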(event Custom|GameStart
  (Variables|Default|SetTimer 15)
  (Utilities|Time|SetTimerbyFunctionName 0 "CountDown" 1.0 true))

(event EventTick
  (params (DeltaSeconds :type Float%20%28single-precision%29))
  (if (< (Variables|Default|GetTimer) 1)
    (if (Variables|Default|GetGameIsStart)
      (bind _returnvalue (UserInterface|CreateWidget "/Game/Blueprints/Widgets/GameOverMenu.GameOverMenu_C"))
      (UserInterface|Viewport|AddtoViewport _returnvalue 0)
      (Variables|/Script/Engine.PlayerController|SetbShowMouseCursor (Game|GetPlayerController 0) true)
      (Variables|Default|SetGameIsStart false))))

(fn ConstructionScript)

(fn OnRepGameStartTimer)

(fn OnRepRandomTimerValue1)

(fn CountDown
  (if (> (Variables|Default|GetTimer) 0)
    (Variables|Default|SetTimer (+ (Variables|Default|GetTimer) -1))))